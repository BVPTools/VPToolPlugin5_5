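; Probe actor that measures floor height beneath its Arrow component for a camera manager.
; MesureFloor stores the camera manager reference, then line-traces straight down against static and dynamic world objects with debug drawing.
; The result sets the manager's HasProbed and FloorHeight, falling back to NullHeight on a miss, and prints to screen.
; TestProbe runs the same trace on the stored reference after raising the texture streaming pool size by console command.
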(event Custom|MesureFloor
  (params (CameraRef :type BP%20Camera%20Manager%20Object%20Reference))
  (bind _arrow (Variables|Default|GetArrow))
  (bind _returnvalue (Transformation|GetWorldLocation _arrow))
  (Variables|Default|SetCamera%20Manager%20Ref CameraRef)
  (bind (_outhit _returnvalue_2) (Collision|LineTraceForObjects _returnvalue (+ _returnvalue (* "0,0,1.000000" -2e+05)) (Utilities|Array|MakeArray "ObjectTypeQuery1" "ObjectTypeQuery2") false 0 "ForDuration"))
  (if (Utilities|IsValid (Variables|Default|GetCamera%20Manager%20Ref))
    (if _returnvalue_2
      (Variables|/BelindaVPTool/Blueprints/BP_CameraManager.BP_CameraManager_C|SetHasProbed? (Variables|Default|GetCamera%20Manager%20Ref) true)
      (bind _output_get (Variables|/BelindaVPTool/Blueprints/BP_CameraManager.BP_CameraManager_C|SetFloor%20Height (Variables|Default|GetCamera%20Manager%20Ref) (.Z (Math|Vector|BreakVector (.Location (Collision|BreakHitResult _outhit))))))
      (Development|PrintString (Utilities|String|Append "Floor height : " (Utilities|String|ToString(Float) _output_get)) true true "(R=0.000000,G=0.660000,B=1.000000,A=1.000000)" 1e+01 "FloorHeight")
      (else
        (Variables|/BelindaVPTool/Blueprints/BP_CameraManager.BP_CameraManager_C|SetHasProbed? (Variables|Default|GetCamera%20Manager%20Ref) false)
        (Variables|/BelindaVPTool/Blueprints/BP_CameraManager.BP_CameraManager_C|SetFloor%20Height (Variables|Default|GetCamera%20Manager%20Ref) (Variables|Default|GetNull%20Height))
        (Development|PrintString "No floor hit" true true "(R=1.000000,G=0.000000,B=0.000000,A=1.000000)" 1e+01 "FloorHeight")))))

(event Custom|TestProbe
  (bind _arrow (Variables|Default|GetArrow))
  (bind _returnvalue (Transformation|GetWorldLocation _arrow))
  (Development|ExecuteConsoleCommand "r.Streaming.PoolSize 5000" 0)
  (bind (_outhit _returnvalue_2) (Collision|LineTraceForObjects _returnvalue (+ _returnvalue (* "0,0,1.000000" -2e+05)) (Utilities|Array|MakeArray "ObjectTypeQuery1" "ObjectTypeQuery2") false 0 "ForDuration"))
  (if (Utilities|IsValid (Variables|Default|GetCamera%20Manager%20Ref))
    (if _returnvalue_2
      (Variables|/BelindaVPTool/Blueprints/BP_CameraManager.BP_CameraManager_C|SetHasProbed? (Variables|Default|GetCamera%20Manager%20Ref) true)
      (bind _output_get (Variables|/BelindaVPTool/Blueprints/BP_CameraManager.BP_CameraManager_C|SetFloor%20Height (Variables|Default|GetCamera%20Manager%20Ref) (.Z (Math|Vector|BreakVector (.Location (Collision|BreakHitResult _outhit))))))
      (Development|PrintString (Utilities|String|Append "Floor height : " (Utilities|String|ToString(Float) _output_get)) true true "(R=0.000000,G=0.660000,B=1.000000,A=1.000000)" 1e+01 "FloorHeight")
      (else
        (Variables|/BelindaVPTool/Blueprints/BP_CameraManager.BP_CameraManager_C|SetHasProbed? (Variables|Default|GetCamera%20Manager%20Ref) false)
        (Variables|/BelindaVPTool/Blueprints/BP_CameraManager.BP_CameraManager_C|SetFloor%20Height (Variables|Default|GetCamera%20Manager%20Ref) (Variables|Default|GetNull%20Height))
        (Development|PrintString "No floor hit" true true "(R=1.000000,G=0.000000,B=0.000000,A=1.000000)" 1e+01 "FloorHeight")))))

(fn ConstructionScript)