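; Virtual production camera manager that drives BP_MainCameraRobot's cine camera and a turntable from Live Link FreeD data.
; FreeD movement poses the camera with optional flip, while turntable yaw rotates this actor and optionally counter-rotates its height-scaled skeletal mesh.
; SetupCamera has BP_Probe measure the floor, then aligns the camera at offset focus distance and attaches it to the root to follow the turntable.
; Helpers handle nodal offsets, floor placement and debug drawing.
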(event OnLiveLinkUpdated(FreeDMovement)
  (params (DeltaTime :type Float%20%28single-precision%29))
  (bind _maincameraref (Variables|Cam_config|GetMainCameraRef))
  (bind _returnvalue (Class|CineCameraActor|GetCineCameraComponent _maincameraref))
  ;[0 0 1 1 32] CAM 1 - FREED MOVEMENT
  (Utilities|CheckCam
    (:Found
      (bind _dataresult (|EvaluateLiveLinkFramewithSpecificRole "(Name=\"Camera 1\")" "/Script/LiveLinkInterface.LiveLinkCameraRole")
        (:then
          (Transformation|SetRelativeLocationAndRotation _returnvalue (.Location (Utilities|GetOffsetedTransform (.Transform (Utilities|Struct|BreakLiveLinkCameraFrameData (.FrameData (Utilities|Struct|BreakLiveLinkCameraBlueprintData _dataresult)))))) (select (Variables|Default|GetflipCam) (Math|Rotator|MakeRotator (+ (.Roll (Math|Rotator|BreakRotator (.Rotation (Utilities|GetOffsetedTransform (.Transform (Utilities|Struct|BreakLiveLinkCameraFrameData (.FrameData (Utilities|Struct|BreakLiveLinkCameraBlueprintData _dataresult)))))))) 1.8e+02) (.Pitch (Math|Rotator|BreakRotator (.Rotation (Utilities|GetOffsetedTransform (.Transform (Utilities|Struct|BreakLiveLinkCameraFrameData (.FrameData (Utilities|Struct|BreakLiveLinkCameraBlueprintData _dataresult)))))))) (.Yaw (Math|Rotator|BreakRotator (.Rotation (Utilities|GetOffsetedTransform (.Transform (Utilities|Struct|BreakLiveLinkCameraFrameData (.FrameData (Utilities|Struct|BreakLiveLinkCameraBlueprintData _dataresult))))))))) (.Rotation (Utilities|GetOffsetedTransform (.Transform (Utilities|Struct|BreakLiveLinkCameraFrameData (.FrameData (Utilities|Struct|BreakLiveLinkCameraBlueprintData _dataresult))))))) false false)
          (Variables|Cam_config|SetTrackingLocation (+ (Transformation|GetWorldLocation _returnvalue) (* (Math|Vector|GetForwardVector (Class|CineCameraActor|GetCineCameraComponent (Variables|Cam_config|GetMainCameraRef))) (CallFunction|GetOffsetedFD (Variables|/Script/CinematicCamera.CineCameraComponent|GetCurrentFocusDistance _returnvalue)))))
          (if (Variables|Cam_Debug|GetDrawDebug?)
            (Rendering|Debug|DrawDebugSphere (Variables|Cam_config|GetTrackingLocation) 2.0 6 "(R=1.000000,G=0.000000,B=0.000000,A=1.000000)" 0.1 0.2)))))))

(event OnLiveLinkUpdated(FreeDTurnTable)
  (params (DeltaTime :type Float%20%28single-precision%29))
  (bind _skeletalmesh (Variables|Default|GetSkeletalMesh))
  (bind _relativerotation (Variables|/Script/Engine.SceneComponent|GetRelativeRotation _skeletalmesh))
  ;[0 0 1 1 32] CAM2 - FREED TURNTABLE
  (bind _dataresult (|EvaluateLiveLinkFramewithSpecificRole "(Name=\"Camera 2\")" "/Script/LiveLinkInterface.LiveLinkCameraRole")
    (:then
      (Variables|TTVals|Setx (* (|((({6FCC90EB-42CD-3CAC-CCB9-EE8584E4372A}*(cosd(z)))-({A04578FE-448C-D493-7879-64AAA39AAB2B}*(sind(z))))-{A04578FE-448C-D493-7879-64AAA39AAB2B}) (.Yaw (Math|Rotator|BreakRotator (.Rotation (Math|Transform|BreakTransform (.Transform (Utilities|Struct|BreakLiveLinkCameraFrameData (.FrameData (Utilities|Struct|BreakLiveLinkCameraBlueprintData _dataresult))))))))) -1.0))
      (Variables|TTVals|Sety (* (|((({A04578FE-448C-D493-7879-64AAA39AAB2B}*(sind(z)))+({6FCC90EB-42CD-3CAC-CCB9-EE8584E4372A}*(cosd(z))))-{6FCC90EB-42CD-3CAC-CCB9-EE8584E4372A}) (.Yaw (Math|Rotator|BreakRotator (.Rotation (Math|Transform|BreakTransform (.Transform (Utilities|Struct|BreakLiveLinkCameraFrameData (.FrameData (Utilities|Struct|BreakLiveLinkCameraBlueprintData _dataresult))))))))) -1.0))
      (Transformation|SetActorRotation (Math|Rotator|MakeRotator (.Roll (Math|Rotator|BreakRotator (.Rotation (Math|Transform|BreakTransform (.Transform (Utilities|Struct|BreakLiveLinkCameraFrameData (.FrameData (Utilities|Struct|BreakLiveLinkCameraBlueprintData _dataresult)))))))) (.Pitch (Math|Rotator|BreakRotator (.Rotation (Math|Transform|BreakTransform (.Transform (Utilities|Struct|BreakLiveLinkCameraFrameData (.FrameData (Utilities|Struct|BreakLiveLinkCameraBlueprintData _dataresult)))))))) (+ (+ (* (.Yaw (Math|Rotator|BreakRotator (.Rotation (Math|Transform|BreakTransform (.Transform (Utilities|Struct|BreakLiveLinkCameraFrameData (.FrameData (Utilities|Struct|BreakLiveLinkCameraBlueprintData _dataresult)))))))) -1.0) (Variables|Default|GetStartYawRotation)) (Variables|Default|GetStartRotationOffset))))
      (if (Variables|Default|GetuseCamRotation?)
        (Transformation|SetRelativeRotation _skeletalmesh (Math|Rotator|MakeRotator (.roll _relativerotation) (.pitch _relativerotation) (+ (- 3.6e+02 (+ (+ (* (.Yaw (Math|Rotator|BreakRotator (.Rotation (Math|Transform|BreakTransform (.Transform (Utilities|Struct|BreakLiveLinkCameraFrameData (.FrameData (Utilities|Struct|BreakLiveLinkCameraBlueprintData _dataresult)))))))) -1.0) (Variables|Default|GetStartYawRotation)) (Variables|Default|GetStartRotationOffset))) 9e+01)) false false)
        (else
          (Transformation|SetRelativeRotation _skeletalmesh (Math|Rotator|MakeRotator (.roll _relativerotation) (.pitch _relativerotation) 9e+01) false false))))))

(event Custom|SetupCamera
  (bind _nodal_offset (Variables|Cam_config|GetNodal%20Offset))
  ;[1 0.1574 0 1 32] Camera Setup
  (Utilities|CheckProbe
    (:Found
      (Default|MesureFloor (Variables|CamProbe|GetProbeRef) self)
      (Utilities|CheckCam
        (:Found
          ;;[0 0 0 1 32] 1 - Calcul pos desiree
          (Variables|Cam_config|SetCameraDesiredPostion (- (Transformation|GetActorLocation) (- (* (Math|Vector|GetForwardVector (Transformation|GetActorRotation)) (CallFunction|GetOffsetedFD (Variables|/Script/CinematicCamera.CineCameraComponent|GetCurrentFocusDistance (Class|CineCameraActor|GetCineCameraComponent (Variables|Cam_config|GetMainCameraRef))))) (select (Variables|Cam_config|GetUseNodal?) (Math|Vector|MakeVector (.x _nodal_offset) (.y _nodal_offset) (.z _nodal_offset)) "0, 0, 0"))))
          ;;[1 1 1] Comment
          (bind _output_get (Variables|Cam_config|SetYawDesiredOffset (- (.Yaw (Math|Rotator|BreakRotator (Transformation|GetActorRotation))) (.yaw (Transformation|GetWorldRotation (Class|CineCameraActor|GetCineCameraComponent (Variables|Cam_config|GetMainCameraRef)))))))
          (Transformation|AddLocalRotation (Variables|/Script/Engine.CameraActor|GetSceneComponent (Variables|Cam_config|GetMainCameraRef)) (Math|Rotator|MakeRotator 0.0 0.0 _output_get) false false)
          (Transformation|AddLocalOffset (Variables|/Script/Engine.CameraActor|GetSceneComponent (Variables|Cam_config|GetMainCameraRef)) (- (Math|Transform|InverseTransformLocation (Transformation|GetActorTransform (Variables|Cam_config|GetMainCameraRef)) (Variables|Cam_config|GetCameraDesiredPostion)) (Variables|/Script/Engine.SceneComponent|GetRelativeLocation (Class|CineCameraActor|GetCineCameraComponent (Variables|Cam_config|GetMainCameraRef)))) false false)
          (Transformation|AttachComponentToComponent (Variables|Cam_config|GetMainCameraRef) (Variables|Default|GetDefaultSceneRoot) "None" "KeepWorld" "KeepWorld" "KeepWorld" true))))))

(event Custom|SetDebug
  (Variables|Cam_Debug|SetDrawDebug? (not (Variables|Cam_Debug|GetDrawDebug?))))

(event Custom|SetNodal
  (bind _output_get (Variables|Cam_config|SetUseNodal? (not (Variables|Cam_config|GetUseNodal?))))
  (Development|PrintString (Utilities|String|Append "Nodal SetTo : " (Utilities|String|ToString(Boolean) _output_get))))

(event Custom|Reset
  (Variables|Cam_config|SetUseNodal? false)
  (Utilities|FlowControl|DelayUntilNextTick)
  (Utilities|CheckProbe
    (:Found
      (Default|MesureFloor (Variables|CamProbe|GetProbeRef) self))))

(event Custom|Distance
  (bind _maincameraref (Variables|Cam_config|GetMainCameraRef))
  (bind _returnvalue (Class|CineCameraActor|GetCineCameraComponent _maincameraref))
  (bind _returnvalue_2 (Transformation|GetWorldLocation _returnvalue))
  (bind _outhit (Collision|LineTraceForObjects _returnvalue_2 (+ _returnvalue_2 (* (Math|Vector|GetForwardVector (Class|CineCameraActor|GetCineCameraComponent (Variables|Cam_config|GetMainCameraRef))) 1e+05)) (Utilities|Array|MakeArray "ObjectTypeQuery1" "ObjectTypeQuery2") false 0 "ForDuration" true "(R=1.000000,G=0.000000,B=0.000000,A=1.000000)" "(R=0.000000,G=1.000000,B=0.000000,A=1.000000)" 3e+01))
  (Development|PrintString (Utilities|String|ToString(Float) (.Distance (Collision|BreakHitResult _outhit))))
  (Development|PrintString (Utilities|String|Append "Dist : " (Utilities|String|ToString(Float) (Math|Vector|Distance(Vector) _returnvalue_2 (Variables|Cam_config|GetTrackingLocation))))))

(event Custom|PlacePawn
  (bind _returnvalue (Transformation|GetActorLocation))
  (bind _skeletalmesh (Variables|Default|GetSkeletalMesh))
  (bind _returnvalue_2 (Transformation|GetWorldLocation _skeletalmesh))
  (bind (_outhit _returnvalue_3) (Collision|LineTraceForObjects _returnvalue (+ _returnvalue (* (Transformation|GetActorUpVector) -1e+06)) (Utilities|Array|MakeArray "ObjectTypeQuery1" "ObjectTypeQuery2") false 0 "ForDuration" true "(R=1.000000,G=0.000000,B=0.000000,A=1.000000)" "(R=0.000000,G=1.000000,B=0.000000,A=1.000000)" 6e+01))
  (if _returnvalue_3
    (Transformation|SetWorldLocation _skeletalmesh (Math|Vector|MakeVector (.x _returnvalue_2) (.y _returnvalue_2) (.Z (Math|Vector|BreakVector (.Location (Collision|BreakHitResult _outhit))))) false false)))

(event Custom|PlaceAtFocusDistance
  (bind _returnvalue (Math|Vector|GetForwardVector "0, 0, 0"))
  (bind _returnvalue_2 (Actor|GetActorOfClass "/BelindaVPTool/Blueprints/BP_MainCameraRobot.BP_MainCameraRobot_C"))
  (Rendering|Debug|DrawDebugSphere (+ "" (* (Math|Vector|MakeVector (.x _returnvalue) (.y _returnvalue) (.z _returnvalue)) (Variables|/Script/CinematicCamera.CineCameraComponent|GetCurrentFocusDistance (Class|CineCameraActor|GetCineCameraComponent _returnvalue_2)))) 1e+01 12 "(R=1.000000,G=0.011906,B=0.000000,A=1.000000)" 2e+01)
  (bind _returnvalue_3 (Actor|GetActorOfClass "BP_CameraManager_C"))
  (Utilities|IsValid _returnvalue_3
    (:Is%20Valid
      (Transformation|SetActorLocation _returnvalue_3 (+ "" (* (Math|Vector|MakeVector (.x _returnvalue) (.y _returnvalue) (.z _returnvalue)) (Variables|/Script/CinematicCamera.CineCameraComponent|GetCurrentFocusDistance (Class|CineCameraActor|GetCineCameraComponent _returnvalue_2)))) false false))))

(event Custom|SetUseNodal
  (params (NodalOffset :type Float%20%28double-precision%29))
  (Variables|Default|SetZNodalOffset NodalOffset))

(fn ConstructionScript
  (Transformation|SetRelativeScale3D (Variables|Default|GetSkeletalMesh) (Math|Conversions|ToVector(Float) (/ (Variables|Default|GetCharacterHeight) 181.0))))

(fn GetNormalizedFocus
  (return (CallFunction|GetOffsetedFD (Variables|/Script/CinematicCamera.CineCameraComponent|GetCurrentFocusDistance (Class|CineCameraActor|GetCineCameraComponent (Variables|Cam_config|GetMainCameraRef))))))

(fn GetOffsetedFD
  (params (FocusDistance :type Float%20%28double-precision%29))
  (return (- FocusDistance (Variables|Default|GetZNodalOffset))))

(fn NewFunction)

(fn TestFnct
  (CallFunction|SetupCamera)
  (Development|PrintString "CPP Fnct call !!!!!" true true "(R=0.000000,G=0.660000,B=1.000000,A=1.000000)" 2e+01))