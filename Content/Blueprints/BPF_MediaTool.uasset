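; Blueprint function library for a media tool, whose SpawnRig function, as shown, only clears the level and spawns nothing.
; It removes leftover probe, camera robot and camera manager actors, then base lighting, sky, fog, cloud, Ultra Dynamic Sky/Weather and PlayerStart actors.
; CleanAssetByClass does the work by destroying every actor of a given class.
; Sky spheres are found separately by matching StaticMeshActor meshes against SM_SkySphere.
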(fn SpawnRig
  (bind ___worldcontext (LocalVariables|Get__WorldContext))
  (bind ___worldcontext_2 (LocalVariables|Get__WorldContext))
  (bind ___worldcontext_3 (LocalVariables|Get__WorldContext))
  (Utilities|FlowControl|Sequence
    (:then_0
      ;[0 0 0 1 40] CLEAN
      ;;[0 0 0 1 25] Clean remaining Tool elements
      (Utilities|FlowControl|Sequence
        (:then_0
          (CallFunction|CleanAssetbyClass "/BelindaVPTool/Blueprints/BP_Probe.BP_Probe_C" ___worldcontext_2))
        (:then_1
          (CallFunction|CleanAssetbyClass 0 ___worldcontext_2))
        (:then_2
          (CallFunction|CleanAssetbyClass 0 ___worldcontext_2))
        (:then_3
          (CallFunction|CleanAssetbyClass "/BelindaVPTool/Blueprints/BP_MainCameraRobot.BP_MainCameraRobot_C" ___worldcontext_2))
        (:then_4
          (CallFunction|CleanAssetbyClass "/BelindaVPTool/Blueprints/BP_CameraManager.BP_CameraManager_C" ___worldcontext_2))
        (:then_5
          ;;[0 0 0 1 25] Clean base light
          (Utilities|FlowControl|Sequence
            (:then_0
              (CallFunction|CleanAssetbyClass "/Script/Engine.DirectionalLight" ___worldcontext))
            (:then_1
              (CallFunction|CleanAssetbyClass "/Script/Engine.ExponentialHeightFog" ___worldcontext))
            (:then_2
              (CallFunction|CleanAssetbyClass "/Script/Engine.SkyAtmosphere" ___worldcontext))
            (:then_3
              (CallFunction|CleanAssetbyClass "/Script/Engine.SkyLight" ___worldcontext))
            (:then_4
              (CallFunction|CleanAssetbyClass "/Script/Engine.VolumetricCloud" ___worldcontext))
            (:then_5
              (CallFunction|CleanAssetbyClass "/Script/Engine.PlayerStart" ___worldcontext)
              (CallFunction|CleanAssetbyClass "/Script/Engine.PlayerStart" ___worldcontext_3)
              (CallFunction|CleanAssetbyClass "/BelindaVPTool/UltraDynamicSky/Blueprints/Ultra_Dynamic_Sky.Ultra_Dynamic_Sky_C" ___worldcontext_3)
              (CallFunction|CleanAssetbyClass "/BelindaVPTool/UltraDynamicSky/Blueprints/Ultra_Dynamic_Weather.Ultra_Dynamic_Weather_C" ___worldcontext_3))
            (:then_6
              (bind _outactors (Actor|GetAllActorsOfClass (LocalVariables|Get__WorldContext) "/Script/Engine.StaticMeshActor"))
              (for _array_element _outactors
                (if (or (== (Variables|/Script/Engine.StaticMeshComponent|GetStaticMesh (Variables|/Script/Engine.StaticMeshActor|GetStaticMeshComponent _array_element)) "/Engine/MapTemplates/Sky/SM_SkySphere.SM_SkySphere") (== (Variables|/Script/Engine.StaticMeshComponent|GetStaticMesh (Variables|/Script/Engine.StaticMeshActor|GetStaticMeshComponent _array_element)) "/Engine/EngineSky/SM_SkySphere.SM_SkySphere"))
                  (Actor|DestroyActor _array_element))))))))))

(fn CleanAssetbyClass
  (params (ActorClass :type Actor%20Class%20Reference))
  (bind _outactors (Actor|GetAllActorsOfClass (LocalVariables|Get__WorldContext) ActorClass))
  (for _array_element _outactors
    (Actor|DestroyActor _array_element))
  (return))