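; Virtual production turntable actor that rotates with the inverted yaw from a Live Link camera-role subject.
; On each Live Link update it also copies the CineCamera's FOV to its SceneCapture2D and writes the turntable's camera-space depth to a Material Parameter Collection.
; It places an optional plane at the camera's focus distance, scaled from the FOV to fill a 16:9 frame.
; Debug printing is optional.
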(event OnLiveLinkUpdated(LiveLinkComponentController)
  (params (DeltaTime :type Float%20%28single-precision%29))
  (Utilities|FlowControl|Sequence
    (:then_0
      (bind _dataresult (|EvaluateLiveLinkFramewithSpecificRole "(Name=\"Camera 2\")" "/Script/LiveLinkInterface.LiveLinkCameraRole")
        (:then
          (Transformation|SetActorRotation (Math|Rotator|MakeRotator 0.0 0.0 (* (.yaw (.Rotation (Math|Transform|BreakTransform (.Transform (Utilities|Struct|BreakLiveLinkCameraFrameData (.FrameData (Utilities|Struct|BreakLiveLinkCameraBlueprintData _dataresult))))))) -1.0)))
          (if (Variables|Default|GetPrintDebug?)
            (Development|PrintString (Utilities|String|Append "Turntable rotation :" (Utilities|String|ToString(Float) (.yaw (.Rotation (Math|Transform|BreakTransform (.Transform (Utilities|Struct|BreakLiveLinkCameraFrameData (.FrameData (Utilities|Struct|BreakLiveLinkCameraBlueprintData _dataresult))))))))) true true "(R=0.000000,G=0.660000,B=1.000000,A=1.000000)" 2.0 "TTloc")))))
    (:then_1
      (bind _returnvalue (Actor|GetActorOfClass "/Script/CinematicCamera.CineCameraActor"))
      (Variables|Default|SetCineCamComp (Class|CineCameraActor|GetCineCameraComponent _returnvalue))
      (bind _output_get (Variables|/Script/Engine.SceneCaptureComponent2D|SetFOVAngle (Actor|GetComponentbyClass _returnvalue "/Script/Engine.SceneCaptureComponent2D") (Variables|/Script/Engine.CameraComponent|GetFieldOfView (Variables|Default|GetCineCamComp))))
      (Variables|Default|SetFOV _output_get)
      (Variables|Default|SetDistance (CallFunction|ComputeDistance))
      (Rendering|Material|SetScalarParameterValue (Variables|Default|GetMPC) (Utilities|Name|MakeLiteralName "Distance") (Variables|Default|GetOffsetedDistance) :!class /Script/Engine.KismetMaterialLibrary)
      (if (Variables|Default|GetPrintDebug?)
        (Development|PrintString (Utilities|String|Append "Distance : " (Utilities|String|ToString(Float) (Variables|Default|GetDistance))) true true "(R=0.000000,G=0.660000,B=1.000000,A=1.000000)" 2.0 "TTDist")))
    (:then_2
      (bind _plane (Variables|Default|GetPlane)
        (:then
          (Transformation|SetRelativeLocation (Variables|/Script/Engine.StaticMeshActor|GetStaticMeshComponent _plane) (Math|Vector|MakeVector (Variables|/Script/CinematicCamera.CineCameraComponent|GetCurrentFocusDistance (Variables|Default|GetCineCamComp)) 0.0 0.0) false false)
          (Variables|Default|SetScaleY (* (/ (* (* (Math|Trig|Tan(Radians) (/ (Math|Trig|DegreesToRadians (Variables|Default|GetFOV)) 2.0)) (Variables|/Script/CinematicCamera.CineCameraComponent|GetCurrentFocusDistance (Variables|Default|GetCineCamComp))) 2.0) 1e+02) (/ 9.0 16.0)))
          (Variables|Default|SetScaleX (/ (* (* (Math|Trig|Tan(Radians) (/ (Math|Trig|DegreesToRadians (Variables|Default|GetFOV)) 2.0)) (Variables|/Script/CinematicCamera.CineCameraComponent|GetCurrentFocusDistance (Variables|Default|GetCineCamComp))) 2.0) 1e+02))
          (Transformation|SetRelativeScale3D (Variables|/Script/Engine.StaticMeshActor|GetStaticMeshComponent (Variables|Default|GetPlane)) (Math|Vector|MakeVector (Variables|Default|GetScaleX) (Variables|Default|GetScaleY) 1.0)))
        (:else)))))

(fn ConstructionScript)

(fn ComputeDistance
  (bind _returnvalue (Transformation|GetActorTransform))
  (bind _cinecamcomp (Variables|Default|GetCineCamComp))
  (bind _returnvalue_2 (Transformation|GetWorldTransform _cinecamcomp))
  (bind _returnvalue_3 (Math|Transform|InverseTransformLocation _returnvalue_2 (.location _returnvalue)))
  (bind _returnvalue_4 (Math|Float|Absolute(Float) (.x _returnvalue_3)))
  (Variables|Default|SetOffsetedDistance _returnvalue_4)
  (return (+ _returnvalue_4 (.focusoffset (Variables|/Script/CinematicCamera.CineCameraComponent|GetFocusSettings _cinecamcomp)))))