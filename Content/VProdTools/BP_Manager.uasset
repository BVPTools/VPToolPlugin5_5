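; Virtual production manager that positions a BP_Turntable and a CineCameraActor around a shared TargetLocation through four events.
; It moves the turntable to the target and places the camera back along world X by its focus distance, compensating for the component's X/Z offset.
; Attach and detach events parent the camera to the turntable or release it, keeping world transforms.
; The attach guard checks the manager's own parent, not the camera's.
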(event Custom|Setup%20Camera
  (bind _returnvalue (Actor|GetActorOfClass "/Script/CinematicCamera.CineCameraActor"))
  (bind _output_get (Variables|Default|SetTargetLocation_WithFD (Utilities|Operators|Subtract (Variables|Default|GetTargetLocation) (Math|Vector|MakeVector (Variables|/Script/CinematicCamera.CineCameraComponent|GetCurrentFocusDistance (Class|CineCameraActor|GetCineCameraComponent _returnvalue)) 0.0 0.0) (Math|Vector|MakeVector (.x (Variables|/Script/Engine.SceneComponent|GetRelativeLocation (Class|CineCameraActor|GetCineCameraComponent _returnvalue))) 0.0 (.z (Variables|/Script/Engine.SceneComponent|GetRelativeLocation (Class|CineCameraActor|GetCineCameraComponent _returnvalue)))))))
  (Transformation|SetActorLocation _returnvalue _output_get false false))

(event Custom|DetachCamera
  (bind _returnvalue (Actor|GetActorOfClass "/Script/CinematicCamera.CineCameraActor"))
  (bind _returnvalue_2 (Actor|GetActorOfClass "/BelindaVPTool/VProdTools/BP_Turntable.BP_Turntable_C"))
  (if (== _returnvalue_2 (Actor|GetAttachParentActor _returnvalue))
    (Transformation|DetachFromActor _returnvalue "KeepWorld" "KeepWorld" "KeepWorld")))

(event Custom|SetTurntableLocation
  (bind _returnvalue (Actor|GetActorOfClass "/BelindaVPTool/VProdTools/BP_Turntable.BP_Turntable_C"))
  (Transformation|SetActorLocation _returnvalue (Variables|Default|GetTargetLocation) false false))

(event Custom|AttachCamera
  (bind _returnvalue (Actor|GetActorOfClass "/Script/CinematicCamera.CineCameraActor"))
  (bind _returnvalue_2 (Actor|GetActorOfClass "/BelindaVPTool/VProdTools/BP_Turntable.BP_Turntable_C"))
  (if (not (== _returnvalue_2 (Actor|GetAttachParentActor)))
    (Transformation|AttachActorToActor _returnvalue _returnvalue_2 "None" "KeepWorld" "KeepWorld" "KeepWorld" true)))

(fn ConstructionScript)