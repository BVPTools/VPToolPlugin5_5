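; Composure media plate comp element that takes video input and prepares it for chroma keying with editor color picking.
; RenderCompElement runs the media input, or latest result as fallback, through ProcessPlateForKeying, currently a pass-through hook.
; Valid media input is registered as a separate "ProcessedPlate" pass, leaving freezable inputs intact.
; The plate becomes the picking target before parent transform passes run; the chroma keyer or final result feeds the picker display.
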(event EventBeginPlay)

(event Collision|EventActorBeginOverlap
  (params (OtherActor :type Actor%20Object%20Reference)))

(event EventTick
  (params (DeltaSeconds :type Float%20%28single-precision%29)))

(fn ConstructionScript)

(fn RenderCompElement
  (params (bCameraCutThisFrame :type Boolean))
  ;[1 1 1] 1) Get the media input texture
  (bind (_passresult _returnvalue) (Class|CompositingElement|FindInputPass "/Script/Composure.CompositingMediaInput" "None"))
  (Utilities|IsValid _passresult
    (:Is%20Valid
      ;[0.6038 0.6038 1] 2) Apply optional color correction
      (bind _processedplate (CallFunction|ProcessPlateforKeying _passresult))
      (bind _output_get (LocalVariables|SetMediaInputResult _processedplate))
      (Class|CompositingElement|RegisterPassResult "ProcessedPlate" _output_get true) ; DO NOT set this to overwrite the the input -\nWe could freeze inputs, and this is not an input,\nwe don't want to overwrite it when frozen.
    )
    (:Is%20Not%20Valid
      (bind _processedplate_2 (CallFunction|ProcessPlateforKeying (Class|CompositingElement|GetLatestRenderResult)))
      (LocalVariables|SetMediaInputResult _processedplate_2)))
  ;[0.3185 0.3185 1] 3) Set as chroma color picking target
  (bind _astexture_render_target_2d (Utilities|Casting|CastToTextureRenderTarget2D (LocalVariables|GetMediaInputResult))
    (:then
      (Class|CompositingElement|SetEditorColorPickingTarget _astexture_render_target_2d))
    (:CastFailed
      _))
  ;[0.1329 0.1329 1] 4) Apply transform passes (keying, etc.)
  (bind _returnvalue_2 (|CallParentFunction bCameraCutThisFrame))
  (LocalVariables|SetInternalPipelineResult _returnvalue_2)
  ;[0.03311 0.03311 1] 5) Find chroma keying result
  (bind _passresult_2 (Class|CompositingElement|FindTransformPass "/Script/Composure.MultiPassChromaKeyer" "None"))
  (Utilities|IsValid _passresult_2
    (:Is%20Valid
      ;[0 0 1] 6) Set color picker result image
      (Class|CompositingElement|SetEditorColorPickerDisplayImage _passresult_2))
    (:Is%20Not%20Valid
      (Class|CompositingElement|SetEditorColorPickerDisplayImage (LocalVariables|GetInternalPipelineResult))))
  (return (LocalVariables|GetInternalPipelineResult)))

(fn ProcessPlateforKeying
  (params (RawMediaPlate :type Texture%20Object%20Reference))
  (return RawMediaPlate))