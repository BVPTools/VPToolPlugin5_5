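; BP_NDCam is an nDisplay tools camera Blueprint with utility events for a Live Link-driven camera.
; One event re-links the FreeDFIZ Live Link component to the camera through SetLiveLink, and another resets post-process settings to defaults.
; Others issue a "CAMERA ALIGN" console command or draw a debug forward trace against WorldStatic objects.
; Controller-map editing nodes are unconnected, and the construction script is empty.
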(event Custom|DrawRay
  (bind _cameracomponent (Variables|CameraActor|GetCameraComponent))
  (bind _returnvalue (Transformation|GetWorldLocation _cameracomponent))
  (Collision|LineTraceForObjects _returnvalue (+ _returnvalue (* (Math|Vector|GetForwardVector _cameracomponent) 1e+04)) (Utilities|Array|MakeArray "ObjectTypeQuery1") false 0 "ForDuration" true "(R=1.000000,G=0.000000,B=0.000000,A=1.000000)" "(R=0.000000,G=1.000000,B=0.000000,A=1.000000)" 15.0))

(event Custom|ResetPostProcess
  (Variables|/Script/Engine.CameraComponent|SetPostProcessSettings (Variables|CameraActor|GetCameraComponent) (Utilities|Struct|MakePostProcessSettings)))

(event Custom|FixLiveLink
  (Class|VPToolsLib|SetLiveLink (Variables|Default|GetFreeDFIZ) (Variables|CameraActor|GetCameraComponent))
  (Development|PrintString "FIXED LIVE LINK"))

(event Custom|CustomEvent
  (Development|ExecuteConsoleCommand "CAMERA ALIGN" 0))

(fn ConstructionScript)