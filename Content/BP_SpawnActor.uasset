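; BP_SpawnActor is an actor with an Arrow component that can be shown or hidden, apparently as a spawn point marker.
; The construction script sets the arrow's relative Z to its length times its size, raising it by its scaled length.
; The SetVisible event toggles both visibility and hidden-in-game on the arrow, without propagating to children.
; It holds no spawning logic.
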(event Custom|SetVisible
  (params (visible? :type Boolean))
  (Rendering|SetVisibility (Variables|Default|GetArrow) visible? false)
  (Development|SetHiddeninGame (Variables|Default|GetArrow) (not visible?) false))

(event EventBeginPlay)

(event Collision|EventActorBeginOverlap
  (params (OtherActor :type Actor%20Object%20Reference)))

(event EventTick
  (params (DeltaSeconds :type Float%20%28single-precision%29)))

(fn ConstructionScript
  (bind _arrow (Variables|Default|GetArrow))
  (Transformation|SetRelativeLocation _arrow (Math|Vector|MakeVector 0.0 0.0 (* (Variables|/Script/Engine.ArrowComponent|GetArrowLength _arrow) (Variables|/Script/Engine.ArrowComponent|GetArrowSize _arrow))) false false))